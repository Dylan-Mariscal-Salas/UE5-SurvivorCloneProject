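; Game mode Blueprint that starts background music and sets up the score HUD when play begins.
; BeginPlay spawns the Runningfromevil track as a 2D sound, keeps its audio component, then creates the HUD widget with a zero score.
; It binds to a score-changed delegate, whose handler pushes each new score to the HUD.
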(event Custom|OnChangedScoreDelegateFired
  (params (NewScore :type Integer))
  (Default|SetScore (Variables|Default|GetHUD) NewScore))

(event Custom|PlayBGMusic
  (bind _returnvalue (Audio|SpawnSound2D "/Game/Assets/Sounds/runningfromevil.runningfromevil" 0.3 1.0 0.0 0))
  (Variables|Default|SetMusicAudioComponent _returnvalue))

(event EventBeginPlay
  (CallFunction|PlayBGMusic)
  (bind _returnvalue (UserInterface|CreateWidget "/Game/Blueprints/HUDWidget.HUDWidget_C"))
  (Variables|Default|SetHUD _returnvalue)
  (UserInterface|Viewport|AddtoViewport (Variables|Default|GetHUD) 0)
  (Default|SetScore (Variables|Default|GetHUD))
  (EventDispatchers|BindEventtoScoreChangedDelegate (delegate Custom|OnChangedScoreDelegateFired)))

(fn ConstructionScript)